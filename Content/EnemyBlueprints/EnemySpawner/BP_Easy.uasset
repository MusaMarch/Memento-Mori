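; BP_Easy is an enemy spawner for the easy encounter, triggered once when the first-person character overlaps EasyBox.
; After a short delay it plays the Wave1 timeline, whose event track spawns BPC_EnemyOne AI at random points within SpawnerBox bounds, facing along the Arrow.
; A minute-long delay follows spawning, then every BPC_EnemyOne in the level is killed through CallDeath, including any spawned elsewhere.
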(event `self.EasyBox.OnComponentBeginOverlap`
  (params (OverlappedComponent :type "PrimitiveComponent Object Reference") (OtherActor :type "Actor Object Reference") (OtherComp :type "PrimitiveComponent Object Reference") (OtherBodyIndex :type Integer) (bFromSweep :type Boolean) (SweepResult :type "HitResult Structure (by ref)"))
  (bind _spawnerbox (`self.SpawnerBox`))
  (bind (_origin _boxextent) (`KismetSystemLibrary.GetComponentBounds` _spawnerbox))
  (`/Engine/EditorBlueprintResources/StandardMacros.DoOnce` false
    (:`Completed`
      (cast `/Game/FirstPersonBP/Blueprints/FirstPersonCharacter` OtherActor)
      (`KismetSystemLibrary.Delay` 1.3)
      (`Timeline|Wave1` :!via `PlayFromStart`
        (:`Wave1`
          (`AIBlueprintHelperLibrary.SpawnAIFromClass` "/Game/EnemyBlueprints/Corpse/BPC_EnemyOne.BPC_EnemyOne_C" null (+ (`KismetMathLibrary.MakeVector` (`KismetMathLibrary.RandomFloatInRange` (* (.x _boxextent) -1.0) (.x _boxextent)) (`KismetMathLibrary.RandomFloatInRange` (* (.y _boxextent) -1.0) (.y _boxextent)) (`KismetMathLibrary.RandomFloatInRange` (* (.z _boxextent) -1.0) (.z _boxextent))) (`SceneComponent.K2_GetComponentLocation` _spawnerbox)) (`SceneComponent.K2_GetComponentRotation` (`self.Arrow`)) false null)
          (`KismetSystemLibrary.Delay` 60.0)
          (bind _outactors (`GameplayStatics.GetAllActorsOfClass` "/Game/EnemyBlueprints/Corpse/BPC_EnemyOne.BPC_EnemyOne_C"))
          (for _array_element _outactors
            (`/Game/EnemyBlueprints/Corpse/BPC_EnemyOne.CallDeath` _array_element)))))))

(fn `UserConstructionScript`)